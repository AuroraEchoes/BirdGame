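; BP_FlyPlayer is a player pawn that flies freely along its forward, right and up axes and looks around with yaw and pitch.
; On BeginPlay it adds the IMC_FlyControls Enhanced Input mapping context to its player controller's subsystem.
; Surge, sway and heave actions feed AddMovementInput along actor vectors, while turn actions feed controller yaw and pitch scaled by MouseSensitivity.
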(event `self.ReceiveBeginPlay`
  (bind _asplayer_controller (cast `PlayerController` (`self.GetController`)))
  (`EnhancedInputSubsystemInterface.AddMappingContext` (pcsubsystem `EnhancedInputLocalPlayerSubsystem` _asplayer_controller) "/Game/Inputs/IMC_FlyControls.IMC_FlyControls" 0 (struct)))

(event `EnhancedInput|/Game/Inputs/IA_MoveSurge`
  (params (ActionValue :type "Float (double-precision)") (ElapsedSeconds :type "Float (double-precision)") (TriggeredSeconds :type "Float (double-precision)") (InputAction :type "InputAction Object Reference" :default "/Game/Inputs/IA_MoveSurge.IA_MoveSurge"))
  (:`Triggered`
    (`self.AddMovementInput` (`self.GetActorForwardVector`) ActionValue)))

(event `EnhancedInput|/Game/Inputs/IA_MoveSway`
  (params (ActionValue :type "Float (double-precision)") (ElapsedSeconds :type "Float (double-precision)") (TriggeredSeconds :type "Float (double-precision)") (InputAction :type "InputAction Object Reference" :default "/Game/Inputs/IA_MoveSway.IA_MoveSway"))
  (:`Triggered`
    (`self.AddMovementInput` (`self.GetActorRightVector`) ActionValue)))

(event `EnhancedInput|/Game/Inputs/IA_MoveHeave`
  (params (ActionValue :type "Float (double-precision)") (ElapsedSeconds :type "Float (double-precision)") (TriggeredSeconds :type "Float (double-precision)") (InputAction :type "InputAction Object Reference" :default "/Game/Inputs/IA_MoveHeave.IA_MoveHeave"))
  (:`Triggered`
    (`self.AddMovementInput` (`self.GetActorUpVector`) ActionValue)))

(event `EnhancedInput|/Game/Inputs/IA_TurnYaw`
  (params (ActionValue :type "Float (double-precision)") (ElapsedSeconds :type "Float (double-precision)") (TriggeredSeconds :type "Float (double-precision)") (InputAction :type "InputAction Object Reference" :default "/Game/Inputs/IA_TurnYaw.IA_TurnYaw"))
  (:`Triggered`
    (`self.AddControllerYawInput` (* ActionValue (`self.MouseSensitivity`)))))

(event `EnhancedInput|/Game/Inputs/IA_TurnPitch`
  (params (ActionValue :type "Float (double-precision)") (ElapsedSeconds :type "Float (double-precision)") (TriggeredSeconds :type "Float (double-precision)") (InputAction :type "InputAction Object Reference" :default "/Game/Inputs/IA_TurnPitch.IA_TurnPitch"))
  (:`Triggered`
    (`self.AddControllerPitchInput` (* ActionValue (`self.MouseSensitivity`)))))

(fn `UserConstructionScript`)