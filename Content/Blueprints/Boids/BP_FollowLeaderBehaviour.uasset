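; Boid flocking behaviour that steers a boid toward the leader, which is the player-location actor supplied by its flock.
; GetDesiredDirection returns the normalized vector from the boid to that actor with full weighting when the actor lies within NeighbourRadius.
; Outside that radius it returns a zero direction and zero weight, so the behaviour contributes no steering.
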(fn `GetDesiredDirection`
  (params (Flock :type "BoidFlock Object Reference") (Boid :type "Pawn Object Reference"))
  (returns (ReturnValue :type "BoidBehaviourDirectionInfo Structure"))
  (bind _returnvalue (`Actor.K2_GetActorLocation` Boid))
  (bind _returnvalue_2 (`BoidFlock.GetPlayerLocation` Flock))
  (bind _returnvalue_3 (`Actor.K2_GetActorLocation` _returnvalue_2))
  (bind _returnvalue_4 (<= (`KismetMathLibrary.Vector_Distance` _returnvalue_3 _returnvalue) (`self.NeighbourRadius`)))
  (return (make `BoidBehaviourDirectionInfo` (`KismetMathLibrary.SelectVector` (`KismetMathLibrary.Normal` (- _returnvalue_3 _returnvalue)) (0.0 0.0 0.0) _returnvalue_4) (`KismetMathLibrary.SelectFloat` 1.0 0.0 _returnvalue_4))))