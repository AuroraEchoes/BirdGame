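; BP_CohesionBehaviour is the cohesion rule for a boids flock, steering a boid toward its neighbours.
; GetDesiredDirection sums the offsets from the boid to each actor returned by GetNeighbours, then normalises the total into a direction pointing at their average position.
; It returns that direction with a fixed, neutral relative weighting.
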(fn `GetDesiredDirection`
  (params (Flock :type "BoidFlock Object Reference") (Boid :type "Pawn Object Reference"))
  (returns (ReturnValue :type "BoidBehaviourDirectionInfo Structure"))
  (locals (Cohesion :type "Vector Structure"))
  (for _array_element (`self.GetNeighbours` Flock Boid)
    (set `local.Cohesion` (+ (`local.Cohesion`) (- (`Actor.K2_GetActorLocation` _array_element) (`Actor.K2_GetActorLocation` Boid)))))
  (return (make `BoidBehaviourDirectionInfo` (`KismetMathLibrary.Normal` (`local.Cohesion`)) 1.0)))