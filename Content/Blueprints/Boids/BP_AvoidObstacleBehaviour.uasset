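; BP_AvoidObstacleBehaviour is a boid flocking behaviour that steers a boid away from obstacles.
; GetDesiredDirection asks the Flock for the closest unobstructed direction within NeighbourRadius, sampling 30 points.
; It overshoots that direction away from the boid's forward vector to sharpen the turn.
; Its relative weighting drops to zero when the clear direction nearly matches forward, so it only contributes when a turn is needed.
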(fn `GetDesiredDirection`
  (params (Flock :type "BoidFlock Object Reference") (Boid :type "Pawn Object Reference"))
  (returns (ReturnValue :type "BoidBehaviourDirectionInfo Structure"))
  (locals (SortedDirections :type "NiagaraDataInterfaceArrayFloat3 Object Reference"))
  (bind _returnvalue (`Actor.GetActorForwardVector` (`local.Boid`)))
  (bind _returnvalue_2 (`BoidFlock.GetClosestUnobstructedDirection` Flock Boid (`self.NeighbourRadius`) 30))
  (return (make `BoidBehaviourDirectionInfo` (+ _returnvalue_2 (* (- _returnvalue_2 _returnvalue) 5.0)) (`KismetMathLibrary.SelectFloat` 0.0 1.0 (< (`KismetMathLibrary.Vector_Distance` _returnvalue_2 _returnvalue) 0.05)))))