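; Boid flocking behaviour that steers a boid toward nearby players.
; GetDesiredDirection loops over all players from the Flock and sums unit vectors from the boid to each player within NeighbourRadius, with out-of-range players contributing zero.
; It returns the unnormalized sum as the desired direction with a constant relative weighting, so several nearby players in similar directions give a stronger pull.
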(fn `GetDesiredDirection`
  (params (Flock :type "BoidFlock Object Reference") (Boid :type "Pawn Object Reference"))
  (returns (ReturnValue :type "BoidBehaviourDirectionInfo Structure"))
  (bind _returnvalue (`Actor.K2_GetActorLocation` Boid))
  (for _array_element (`BoidFlock.GetAllPlayers` Flock)
    (bind _returnvalue_2 (`Actor.K2_GetActorLocation` _array_element))
    (bind _returnvalue_3 (<= (`KismetMathLibrary.Vector_Distance` _returnvalue_2 _returnvalue) (`self.NeighbourRadius`)))
    (set `self.FollowPlayersDirection` (+ (`self.FollowPlayersDirection`) (* (`KismetMathLibrary.SelectVector` (`KismetMathLibrary.Normal` (- _returnvalue_2 _returnvalue)) (0.0 0.0 0.0) _returnvalue_3) (`KismetMathLibrary.SelectFloat` 1.0 0.0 _returnvalue_3)))))
  (return (make `BoidBehaviourDirectionInfo` (`self.FollowPlayersDirection`) 1.0)))