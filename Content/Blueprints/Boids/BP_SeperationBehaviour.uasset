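; Boid flocking behaviour that produces a separation steering direction for a boid within its flock.
; GetDesiredDirection sums a Seperation vector for each neighbour from GetNeighbours, using both actor locations, and returns it with a fixed relative weighting.
; The Seperation graph holds a normalized away-from-neighbour vector scaled linearly by closeness within NeighbourRadius, though that expression appears unconnected to any output.
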(fn `GetDesiredDirection`
  (params (Flock :type "BoidFlock Object Reference") (Boid :type "Pawn Object Reference"))
  (returns (ReturnValue :type "BoidBehaviourDirectionInfo Structure"))
  (locals (Seperation :type "Vector Structure"))
  (for _array_element (`self.GetNeighbours` Flock Boid)
    (set `local.Seperation` (+ (`local.Seperation`) (`self.Seperation` (`Actor.K2_GetActorLocation` Boid) (`Actor.K2_GetActorLocation` _array_element)))))
  (return (make `BoidBehaviourDirectionInfo` (`local.Seperation`) 1.0)))