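; BP_BirdPlayer is the player bird Blueprint that drives an on-screen compass pointing toward the goal.
; BeginPlay creates the HUD widget and caches the location of the BP_Goal actor once.
; Each Tick stores the actor's yaw as Bearing and rotates the HUD's GoalMark by the look-at yaw to the goal minus that yaw, keeping the marker relative to the bird's heading.
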(event EventBeginPlay
  ;[0.15 0.15 0.15 0.5] Compass Direction
  (bind _returnvalue (UserInterface|CreateWidget "/Game/UI/HUD.HUD_C" (Game|GetPlayerController 0)))
  (bind _output_get (Variables|Default|SetCompassREF _returnvalue))
  (UserInterface|Viewport|AddtoViewport _output_get 0)
  ;[0.15 0.15 0.15 0.5] Point to Goal Location
  (bind _returnvalue_2 (Actor|GetActorOfClass "/Game/PCG/Blueprints/BP_Goal.BP_Goal_C"))
  (Variables|Default|SetGoalLocation (Transformation|GetActorLocation _returnvalue_2)))

(event Collision|EventActorBeginOverlap
  (params (OtherActor :type Actor%20Object%20Reference))
  ;[0.15 0.15 0.15 0.5] Compass Direction
)

(event EventTick
  (params (DeltaSeconds :type Float%20%28single-precision%29))
  ;[0.15 0.15 0.15 0.5] Compass Direction
  (Variables|Default|SetBearing (.yaw (Transformation|GetActorRotation)))
  ;;[0.15 0.15 0.15 0.5] Rotate to Goal Flag
  (Class|Widget|SetRenderTransformAngle (Variables|/Game/UI/HUD.HUD_C|GetGoalMark (Variables|Default|GetCompassREF)) (- (.yaw (Math|Rotator|FindLookatRotation (Transformation|GetActorLocation) (Variables|Default|GetGoalLocation))) (.yaw (Transformation|GetActorRotation)))))

(fn ConstructionScript)